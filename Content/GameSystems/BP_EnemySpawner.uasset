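; BP_EnemySpawner is a spawner actor that periodically spawns actors of a configured class at its own location, up to a population cap.
; BeginPlay starts a looping five-second timer that calls Spawn.
; Spawn counts every actor of that class in the world and spawns another only while the count is below MaxSpawn, so the cap is shared across all spawners of that class.
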(event EventBeginPlay
  (Utilities|Time|SetTimerbyFunctionName 0 "Spawn" 5.0 true))

(fn ConstructionScript)

(fn Spawn
  (bind _actor_class (Variables|Default|GetActor%20Class))
  (bind _outactors (Actor|GetAllActorsOfClass _actor_class))
  (if (< (Utilities|Array|Length _outactors) (Variables|Default|GetMaxSpawn))
    (Game|SpawnActorfromClass _actor_class (Math|Conversions|ToTransform(Vector) (Transformation|GetActorLocation)) "Undefined" 0 0)
    (return)
    (else
      (return))))